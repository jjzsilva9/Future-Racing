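; BP_CPU_AI is a computer-controlled race vehicle that follows the BP_CPU_Path_Spline.
; Each tick it steers toward a look-ahead spline point and compares speed to a target that decays exponentially with upcoming bend angle.
; It ramps throttle when at or below target, otherwise coasts or brakes based on required speed change.
; Finish-gate overlaps count laps, reporting race time to AIRacePlayerController from the fourth onward.
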(event EventBeginPlay
  (bind _outactors (Actor|GetAllActorsOfClasswithTag "/Game/Variant_TimeTrial/Blueprints/BP_TimeTrialTrackGate.BP_TimeTrialTrackGate_C" "Finish"))
  (for _array_element _outactors
    (Development|PrintString (Utilities|GetDisplayName _array_element))
    (Variables|Default|SetfinishGate (Utilities|Array|Get(acopy) _outactors))
    (bind _returnvalue (Actor|GetActorOfClass "/Game/CPU/BP_CPU_Path_Spline.BP_CPU_Path_Spline_C"))
    (Variables|Default|SetPathSpline _returnvalue)
    (Variables|Default|SetraceStartTime (Utilities|Time|GetGameTimeinSeconds))))

(event EventTick
  (params (DeltaSeconds :type Float%20%28single-precision%29))
  (bind _steeringval (CallFunction|Steer))
  (Class|ChaosVehicleMovementComponent|SetSteeringInput (Variables|Default|GetVehicleMovementComponent) _steeringval)
  (CallFunction|AdjustSpeed))

(event Collision|EventActorBeginOverlap
  (params (OtherActor :type Actor%20Object%20Reference))
  (bind _asbp_time_trial_track_gate (Utilities|Casting|CastToBP_TimeTrialTrackGate OtherActor))
  (Development|PrintString (Utilities|String|ToString(Boolean) (== _asbp_time_trial_track_gate (Variables|Default|GetfinishGate))))
  (if (== _asbp_time_trial_track_gate (Variables|Default|GetfinishGate))
    (bind _output_get (Variables|Default|SetlapsCompleted (+ (Variables|Default|GetlapsCompleted) 1)))
    (if (>= _output_get 4)
      (bind _asairace_player_controller (Utilities|Casting|CastToAIRacePlayerController (Game|GetPlayerController 0)))
      (Class|AIRacePlayerController|NotifyAIFinished _asairace_player_controller (- (Utilities|Time|GetGameTimeinSeconds) (Variables|Default|GetraceStartTime))))))

(fn ConstructionScript
  (|CallParentFunction))

(fn Steer
  (bind _returnvalue (Transformation|GetActorLocation))
  (bind _pathspline (Variables|Default|GetPathSpline))
  (bind _spline (Variables|/Game/CPU/BP_CPU_Path_Spline.BP_CPU_Path_Spline_C|GetSpline _pathspline))
  (return (* (|CalculateSteerVal (Math|Rotator|FindLookatRotation _returnvalue (Spline|FindLocationClosesttoWorldLocation _spline (|ToTargetDir (Class|SplineComponent|FindTangentClosesttoWorldLocation _spline _returnvalue "World") _returnvalue) "World")) (Variables|Default|GetmaxSteerRange)) (Math|Float|Max(Float) (Variables|Default|GetsteerSensitivity) 0.0))))

(fn Accelerate
  (bind _output_get (Variables|Default|SetthrottleVal (Math|Float|Clamp(Float) (+ (Variables|Default|GetaccelRate) (Variables|Default|GetthrottleVal)) 0.0 (Variables|Default|GetmaxAccel))))
  (return _output_get))

(fn AdjustSpeed
  (bind (_tangent _scandist) (|GetTangentAtScanDist))
  (bind _vehiclemovementcomponent (Variables|Default|GetVehicleMovementComponent))
  (bind _vehiclemovementcomponent_2 (Variables|Default|GetVehicleMovementComponent))
  (bind _returnvalue (Vehicle|GetForwardSpeed _vehiclemovementcomponent_2))
  (bind _vtarget (|GetTargetSpeed (Math|Vector|DotProduct (Math|Vector|Normalize (Transformation|GetActorForwardVector)) (Math|Vector|Normalize _tangent)))
    (:Exec
      (Math|Float|CompareFloat _vtarget _returnvalue
        (:>
          (bind _throttle (CallFunction|Accelerate :!label _label))
          (Class|ChaosVehicleMovementComponent|SetThrottleInput _vehiclemovementcomponent _throttle)
          (Class|ChaosVehicleMovementComponent|SetBrakeInput _vehiclemovementcomponent 0.0))
        (:==
          (goto _label))
        (:<
          (bind _deltavps (|GetSpeedChangePerSecond _vtarget _returnvalue _scandist)
            (:OutExec
              (if (> _deltavps (Variables|Default|GetnaturalDecel))
                (Class|ChaosVehicleMovementComponent|SetBrakeInput _vehiclemovementcomponent 0.0)
                (else
                  (bind _brakeval (|NormalizeToBrakeRate _deltavps)
                    (:OutExec
                      (Class|ChaosVehicleMovementComponent|SetBrakeInput _vehiclemovementcomponent _brakeval)))))
              (Class|ChaosVehicleMovementComponent|SetThrottleInput _vehiclemovementcomponent 0.0)
              (Variables|Default|SetthrottleVal 0.0))))))))